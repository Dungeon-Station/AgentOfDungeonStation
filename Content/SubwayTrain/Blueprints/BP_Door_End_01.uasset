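; Sliding end door for a subway train, with custom events to open and close it.
; OpenDoor and CloseDoor each slide the EndwallDoor01 component along its relative X axis with a timed MoveComponentTo and play the same sound at the actor's location.
; Any overlap with the Box component triggers CloseDoor, while OpenDoor has no caller within this Blueprint.
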(event `OpenDoor`
  (`GameplayStatics.PlaySoundAtLocation` "/Game/Audio/OpenDoor2.OpenDoor2" (`self.K2_GetActorLocation`) (struct) 1.0 1.0 0.0 null null null null)
  (`KismetSystemLibrary.MoveComponentTo` (`self.endwall_door_01`) (94.0 0.0 0.0) (struct) false false 2.0))

(event `CloseDoor`
  (`GameplayStatics.PlaySoundAtLocation` "/Game/Audio/OpenDoor2.OpenDoor2" (`self.K2_GetActorLocation`) (struct) 1.0 1.0 0.0 null null null null)
  (`KismetSystemLibrary.MoveComponentTo` (`self.endwall_door_01`) (4.0 0.0 0.0) (struct) false false 2.0))

(event `self.Box.OnComponentBeginOverlap`
  (params (OverlappedComponent :type "PrimitiveComponent Object Reference") (OtherActor :type "Actor Object Reference") (OtherComp :type "PrimitiveComponent Object Reference") (OtherBodyIndex :type Integer) (bFromSweep :type Boolean) (SweepResult :type "HitResult Structure (by ref)"))
  (`self.CloseDoor`))

(fn `UserConstructionScript`)