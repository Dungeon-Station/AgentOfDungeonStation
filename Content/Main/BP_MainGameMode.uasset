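; BP_MainGameMode is the main game mode that handles the win and game-over end states.
; Tick polls ClearStage and, once it exceeds a fixed threshold, pauses the game, shows the mouse cursor and adds WBP_Win to the viewport, with no one-shot guard.
; The GameOver event does the same with WBP_GameOver, but neither its caller nor any update to ClearStage appears in this graph.
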(event `self.ReceiveTick`
  (params (DeltaSeconds :type "Float (single-precision)"))
  (bind _returnvalue (`GameplayStatics.GetPlayerController` 0))
  (if (> (`self.ClearStage`) 2)
    (set `PlayerController.bShowMouseCursor` true _returnvalue)
    (`GameplayStatics.SetGamePaused` true)
    (bind _returnvalue_2 (`|CreateWidget` "/Game/Main/WBP_Win.WBP_Win_C" _returnvalue))
    (`UserWidget.AddToViewport` _returnvalue_2 0)))

(event `GameOver`
  (bind _returnvalue (`GameplayStatics.GetPlayerController` 0))
  (`GameplayStatics.SetGamePaused` true)
  (set `PlayerController.bShowMouseCursor` true _returnvalue)
  (bind _returnvalue_2 (`|CreateWidget` "/Game/Main/WBP_GameOver.WBP_GameOver_C" _returnvalue))
  (`UserWidget.AddToViewport` _returnvalue_2 0))

(fn `UserConstructionScript`)