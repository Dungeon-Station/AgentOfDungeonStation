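; Train manager actor that starts a round by running an overhead light sequence.
; The first StartTrigger overlap plays a sound, switches on every light in OverHeadLights and primes AccTime past the Tick threshold.
; Tick switches off and removes the first valid light when AccTime exceeds the threshold, then resets the timer.
; These graphs never increment AccTime, so only that first switch-off fires unless it advances elsewhere.
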(event `self.ReceiveTick`
  (params (DeltaSeconds :type "Float (single-precision)"))
  (bind _overheadlights (`self.OverHeadLights`))
  (bind _output (`|GetArrayItem` _overheadlights))
  (if (`self.StartRound`)
    (if (> (`self.AccTime`) 2.0)
      (if (> (`KismetArrayLibrary.Array_Length` _overheadlights) 0)
        (if (`KismetSystemLibrary.IsValid` _output)
          (`/Game/SubwayTrain/Blueprints/BP_Overheadlight_01.LightOff` _output)
          (set `self.AccTime` 0.0)
          (`KismetArrayLibrary.Array_Remove` _overheadlights))))))

(event `self.StartTrigger.OnComponentBeginOverlap`
  (params (OverlappedComponent :type "PrimitiveComponent Object Reference") (OtherActor :type "Actor Object Reference") (OtherComp :type "PrimitiveComponent Object Reference") (OtherBodyIndex :type Integer) (bFromSweep :type Boolean) (SweepResult :type "HitResult Structure (by ref)"))
  (if (not (`self.StartRound`))
    (set `self.AccTime` 5.0)
    (`GameplayStatics.PlaySound2D` "/Game/Audio/LigthOn.LigthOn" 1.0 1.0 0.0 null null)
    (set `self.StartRound` true)
    (for _array_element (`self.OverHeadLights`)
      (`/Engine/EditorBlueprintResources/StandardMacros.IsValid` _array_element
        (:`Is Valid`
          (`/Game/SubwayTrain/Blueprints/BP_Overheadlight_01.LightOn` _array_element))))))

(fn `UserConstructionScript`)