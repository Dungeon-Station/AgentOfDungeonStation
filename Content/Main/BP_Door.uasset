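; BP_Door is a doorway actor whose two door panels slide when something overlaps their trigger volumes.
; InTrigger1 and InTrigger2 each move their own panel to a fixed relative location over one second with MoveComponentTo, then destroy themselves so they fire only once.
; The second trigger also enables query and physics collision on the WallDoorway15001 component.
; The CloseDoor function is an empty stub.
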(event `self.InTrigger1.OnComponentBeginOverlap`
  (params (OverlappedComponent :type "PrimitiveComponent Object Reference") (OtherActor :type "Actor Object Reference") (OtherComp :type "PrimitiveComponent Object Reference") (OtherBodyIndex :type Integer) (bFromSweep :type Boolean) (SweepResult :type "HitResult Structure (by ref)"))
  (`KismetSystemLibrary.MoveComponentTo` (`self.wall_doorway_door_01`) (0.0 1.0 0.0) (struct) false false 1.0)
  (`ActorComponent.K2_DestroyComponent` (`self.InTrigger1`)))

(event `self.InTrigger2.OnComponentBeginOverlap`
  (params (OverlappedComponent :type "PrimitiveComponent Object Reference") (OtherActor :type "Actor Object Reference") (OtherComp :type "PrimitiveComponent Object Reference") (OtherBodyIndex :type Integer) (bFromSweep :type Boolean) (SweepResult :type "HitResult Structure (by ref)"))
  (`KismetSystemLibrary.MoveComponentTo` (`self.wall_doorway_door_02`) (-150.0 1.0 0.0) (struct) false false 1.0)
  (`PrimitiveComponent.SetCollisionEnabled` (`self.wall_doorway_150_01`) "QueryAndPhysics")
  (`ActorComponent.K2_DestroyComponent` (`self.InTrigger2`)))

(fn `CloseDoor`)

(fn `UserConstructionScript`)