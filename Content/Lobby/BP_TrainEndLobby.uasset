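; BP_TrainEndLobby is a lobby Blueprint, apparently the end section of a train, that exposes functions for switching on its two spotlights.
; OnLight makes both spotlights visible, while FlickerLight has a random 60% chance of showing only SpotLight1 and never hides either.
; The SpotLight call in FlickerLight is disconnected, the event graph and construction script are empty, and nothing in this Blueprint calls either function.
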(event `self.ReceiveBeginPlay`)

(event `self.ReceiveTick`
  (params (DeltaSeconds :type "Float (single-precision)")))

(fn `FlickerLight`
  (if (< (`KismetMathLibrary.RandomFloatInRange` 0.0 1.0) 0.6)
    (`SceneComponent.SetVisibility` (`self.SpotLight1`) true false)))

(fn `OnLight`
  (`SceneComponent.SetVisibility` (`self.SpotLight1`) true false)
  (`SceneComponent.SetVisibility` (`self.SpotLight`) true false))

(fn `UserConstructionScript`)